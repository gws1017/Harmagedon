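; BP_BasicPlayerController is a player controller that handles hotkeys for toggling the debug UI and game menus.
; BeginPlay creates the DebuggingUI widget, which DebugKey1 or Tilde toggles only outside distribution builds.
; Escape or DebugKey2 toggles the first visible screen among inventory, equipment and settings, falling back to the pause menu.
; Those menu instances are not created in this graph, and leftover restart and inventory-initialization nodes are unconnected.
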(event EventBeginPlay
  (bind _returnvalue (UserInterface|CreateWidget "/Game/UI/DebuggingUI.DebuggingUI_C" self))
  (Variables|Default|SetDubggingUIInstance _returnvalue))

(event EventTick
  (params (DeltaSeconds :type Float%20%28single-precision%29)))

(event Input|KeyboardEvents|DebugKey1
  (params (Key :type Key%20Structure :default "None") (ActionValue :type Input%20Action%20Value%20Structure))
  (:Pressed
    (if (not (Class|KismetSystemLibrary|IsPackagedforDistribution))
      (Class|BasicPlayerController|ToggleUI (Variables|Default|GetDubggingUIInstance) true))))

(event Input|KeyboardEvents|DebugKeyI
  (params (Key :type Key%20Structure :default "None") (ActionValue :type Input%20Action%20Value%20Structure)))

(event Input|KeyboardEvents|DebugKey2
  (params (Key :type Key%20Structure :default "None") (ActionValue :type Input%20Action%20Value%20Structure))
  (bind _inventoryuiinstance (Variables|Default|GetInventoryUIInstance))
  (bind _settinguiinstance (Variables|Default|GetSettingUIInstance))
  (bind _equipmentuiinstance (Variables|Default|GetEquipmentUIInstance))
  (:Pressed
    (if (UserInterface|Viewport|IsinViewport _inventoryuiinstance)
      (Class|BasicPlayerController|ToggleUI _inventoryuiinstance true)
      (elif (UserInterface|Viewport|IsinViewport _equipmentuiinstance)
        (Class|BasicPlayerController|ToggleUI _equipmentuiinstance true)
        (elif (UserInterface|Viewport|IsinViewport _settinguiinstance)
          (Class|BasicPlayerController|ToggleUI _settinguiinstance true)
          (else
            (Class|BasicPlayerController|ToggleUI (Variables|Default|GetPasueMenuInstance) true)))))))

(event Input|KeyboardEvents|Tilde
  (params (Key :type Key%20Structure :default "None"))
  (:Pressed
    (if (not (Class|KismetSystemLibrary|IsPackagedforDistribution))
      (Class|BasicPlayerController|ToggleUI (Variables|Default|GetDubggingUIInstance) true))))

(event Input|KeyboardEvents|Escape
  (params (Key :type Key%20Structure :default "None"))
  (bind _inventoryuiinstance (Variables|Default|GetInventoryUIInstance))
  (bind _settinguiinstance (Variables|Default|GetSettingUIInstance))
  (bind _equipmentuiinstance (Variables|Default|GetEquipmentUIInstance))
  (:Pressed
    (if (UserInterface|Viewport|IsinViewport _inventoryuiinstance)
      (Class|BasicPlayerController|ToggleUI _inventoryuiinstance true)
      (elif (UserInterface|Viewport|IsinViewport _equipmentuiinstance)
        (Class|BasicPlayerController|ToggleUI _equipmentuiinstance true)
        (elif (UserInterface|Viewport|IsinViewport _settinguiinstance)
          (Class|BasicPlayerController|ToggleUI _settinguiinstance true)
          (else
            (Class|BasicPlayerController|ToggleUI (Variables|Default|GetPasueMenuInstance) true)))))))

(fn ConstructionScript)